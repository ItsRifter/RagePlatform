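; BP_Mimic is a chest trap that attacks and kills the player who enters its trigger box.
; On overlap it freezes the player, plays a fail sound, then uses timed delays to activate the ABP_Mimic attack animation and knock the player sideways.
; It then sets the player's death animation and reports the death text to RGameInstance.
; The game instance's restart event resets the mimic's animation.
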(event `self.ReceiveBeginPlay`
  ; BeginPlay - Start event
  (bind _asrgame_instance (cast `RGameInstance` (`GameplayStatics.GetGameInstance`)))
  (add `RGameInstance.OnGameRestart` _asrgame_instance (delegate `ResetMimic`)))

(event `ResetMimic`
  ; BeginPlay - Start event
  (bind _asabp_mimic (cast `/Game/Animation_Import/Chest/ABP_Mimic` (`SkeletalMeshComponent.GetAnimInstance` (`self.Mimic_Chest_Attack`))))
  (set `/Game/Animation_Import/Chest/ABP_Mimic.Activate` false _asabp_mimic))

(event `self.Triggerbox.OnComponentBeginOverlap`
  (params (OverlappedComponent :type "PrimitiveComponent Object Reference") (OtherActor :type "Actor Object Reference") (OtherComp :type "PrimitiveComponent Object Reference") (OtherBodyIndex :type Integer) (bFromSweep :type Boolean) (SweepResult :type "HitResult Structure (by ref)"))
  (bind _asbp_rage_character (cast `/Game/Blueprints/Characters/BP_RageCharacter` OtherActor))
  (`/Game/Blueprints/Characters/BP_RageCharacter.FreezePlayer` _asbp_rage_character)
  (`GameplayStatics.PlaySound2D` "/Game/Sounds/RawFiles/Fail.Fail" 1.0 1.0 0.0 null null)
  (bind _asabp_mimic (cast `/Game/Animation_Import/Chest/ABP_Mimic` (`SkeletalMeshComponent.GetAnimInstance` (`self.Mimic_Chest_Attack`))))
  (`KismetSystemLibrary.Delay` 1.25)
  (set `/Game/Animation_Import/Chest/ABP_Mimic.Activate` true _asabp_mimic)
  (`KismetSystemLibrary.Delay` 0.45)
  (`RageCharacter.PlayerFall` _asbp_rage_character (* (`SceneComponent.GetRightVector` (`self.Mimic_Chest_Attack`)) 90.0))
  (bind _asabp_player (cast `/Game/Animation_Import/Player/Animation/ABP_Player` (`SkeletalMeshComponent.GetAnimInstance` (`Character.Mesh` _asbp_rage_character))))
  (set `/Game/Animation_Import/Player/Animation/ABP_Player.DeathType` "NewEnumerator0" _asabp_player)
  (`/Game/Animation_Import/Player/Animation/ABP_Player.DiedABP` _asabp_player)
  (bind _asrgame_instance (cast `RGameInstance` (`GameplayStatics.GetGameInstance`)))
  (`RGameInstance.SetOnPlayerDeath` _asrgame_instance (`self.Death Text`)))

(event `self.Triggerbox.OnComponentEndOverlap`
  (params (OverlappedComponent :type "PrimitiveComponent Object Reference") (OtherActor :type "Actor Object Reference") (OtherComp :type "PrimitiveComponent Object Reference") (OtherBodyIndex :type Integer)))

(fn `UserConstructionScript`)