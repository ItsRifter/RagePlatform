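; BP_Safe is a safe chest actor whose animation reacts to the player's proximity.
; A Box trigger checks overlapping components for the "Player" tag.
; On begin and end overlap it sets the Activate flag on the ABP_Safe anim instance of SafeChest2 to true or false, leaving the animation itself to that Anim Blueprint.
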(event `self.Box.OnComponentBeginOverlap`
  (params (OverlappedComponent :type "PrimitiveComponent Object Reference") (OtherActor :type "Actor Object Reference") (OtherComp :type "PrimitiveComponent Object Reference") (OtherBodyIndex :type Integer) (bFromSweep :type Boolean) (SweepResult :type "HitResult Structure (by ref)"))
  (if (`ActorComponent.ComponentHasTag` OtherComp "Player")
    (bind _asabp_safe (cast `/Game/Animation_Import/Chest/ABP_Safe` (`SkeletalMeshComponent.GetAnimInstance` (`self.Safe_Chest_2`))))
    (set `/Game/Animation_Import/Chest/ABP_Safe.Activate` true _asabp_safe)))

(event `self.Box.OnComponentEndOverlap`
  (params (OverlappedComponent :type "PrimitiveComponent Object Reference") (OtherActor :type "Actor Object Reference") (OtherComp :type "PrimitiveComponent Object Reference") (OtherBodyIndex :type Integer))
  (if (`ActorComponent.ComponentHasTag` OtherComp "Player")
    (bind _asabp_safe (cast `/Game/Animation_Import/Chest/ABP_Safe` (`SkeletalMeshComponent.GetAnimInstance` (`self.Safe_Chest_2`))))
    (set `/Game/Animation_Import/Chest/ABP_Safe.Activate` false _asabp_safe)))

(fn `UserConstructionScript`)