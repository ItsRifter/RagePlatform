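; BP_FinaleChest is the end-of-game chest that ends the run when the player enters its trigger box.
; Overlap freezes the player, aims their view at the chest, and has the game instance finalize game-end data, reset and stop timers, and disable look and pause.
; A delayed sequence plays victory audio, triggers the chest-open animation through its AnimBP, fades the screen, then loads the GameComplete level.
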(event `self.ReceiveBeginPlay`
  (bind _asrgame_instance (cast `RGameInstance` (`GameplayStatics.GetGameInstance`)))
  (set `self.GameInstanceRef` _asrgame_instance))

(event `DoEndSequence`
  (bind _asabp_finale_chest (cast `/Game/Blueprints/Entities/ABP_FinaleChest` (`SkeletalMeshComponent.GetAnimInstance` (`self.SkeletalMesh`))))
  (`GameplayStatics.PlaySound2D` "/Game/Sounds/RawFiles/Victory.Victory" 1.0 1.0 0.0 null null)
  (`KismetSystemLibrary.Delay` 2.25)
  (`/Game/Blueprints/Entities/ABP_FinaleChest.OpenChest` _asabp_finale_chest)
  (`KismetSystemLibrary.Delay` 3.8)
  (`/Game/Blueprints/Characters/BP_RageCharacter.PlayFadeEffect` (`self.PlayerRef`) 0.75)
  (`KismetSystemLibrary.Delay` 4.0)
  (`/Game/Blueprints/Characters/BP_RageCharacter.ResetLookAtTarget` (`self.PlayerRef`))
  (`self.CreateEndGameWidget`))

(event `self.Triggerbox.OnComponentBeginOverlap`
  (params (OverlappedComponent :type "PrimitiveComponent Object Reference") (OtherActor :type "Actor Object Reference") (OtherComp :type "PrimitiveComponent Object Reference") (OtherBodyIndex :type Integer) (bFromSweep :type Boolean) (SweepResult :type "HitResult Structure (by ref)"))
  (bind _asbp_rage_character (cast `/Game/Blueprints/Characters/BP_RageCharacter` OtherActor))
  (bind _output_get (set `self.PlayerRef` _asbp_rage_character))
  (`/Game/Blueprints/Characters/BP_RageCharacter.FreezePlayer` _output_get)
  (`self.DoEndSequence`)
  (`/Game/Blueprints/Characters/BP_RageCharacter.LookAtTarget` _output_get self (0.0 0.0 25.0))
  (`self.SendDataLeaderboard`))

(event `SendDataLeaderboard`
  (bind _gameinstanceref (`self.GameInstanceRef`))
  ;[0.026 0.026 0.026 0.5] LeaderboardData
  (`RGameInstance.SetOnGameEnd` _gameinstanceref)
  (set `RGameInstance.TimeVar` 0.0 _gameinstanceref)
  (set `RGameInstance.GameTimeVar` 0.0 _gameinstanceref)
  (set `RGameInstance.bCanCountGameTime` false _gameinstanceref)
  (set `RGameInstance.bCanCountLevelTime` false _gameinstanceref)
  (set `RGameInstance.bCanLook` false _gameinstanceref)
  (set `RGameInstance.bCanPause` false _gameinstanceref))

(event `CreateEndGameWidget`
  ;[0.026 0.026 0.026 0.5] End Widget
  (`GameplayStatics.OpenLevel` "GameComplete"))

(fn `UserConstructionScript`)