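; Base shooter trap that repeatedly fires pooled particles from its Arrow component.
; BeginPlay starts both a one-shot startup timer and the looping shoot timer, and the startup event sets the looping timer again to offset firing.
; Each shot asks the ObjectPool to spawn at the Arrow's world location and rotation with a set lifetime, rather than creating new actors directly.
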(event `self.ReceiveBeginPlay`
  (`parent.ReceiveBeginPlay`)
  (`KismetSystemLibrary.K2_SetTimerDelegate` (delegate `StartupWait`) (`self.TimeDelay`))
  (bind _returnvalue (`KismetSystemLibrary.K2_SetTimerDelegate` (delegate `FireParticle`) (`self.TimeToShoot`) true :!label _label))
  (set `self.ShootTimer` _returnvalue))

(event `StartupWait`
  (goto _label))

(event `FireParticle`
  (`/Game/Blueprints/Misc/AC_ObjectPool.SpawnFromPool` (`self.ObjectPool`) (`KismetMathLibrary.MakeTransform` (`SceneComponent.K2_GetComponentLocation` (`self.Arrow`)) (`SceneComponent.K2_GetComponentRotation` (`self.Arrow`))) (`self.ParticleLifetime`)))

(fn `UserConstructionScript`)