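; Ceiling collapse trap, a child of a base trap class, that drops a kill box to crush the player.
; When triggered with an active trigger component, the CeilingDrop timeline offsets KillBox downward from its BeginPlay location, scaled by Distance and Speed.
; Reset plays the timeline in reverse, and the parent reset runs when the timeline finishes with the trap not ready.
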(event `self.ReceiveBeginPlay`
  (`parent.ReceiveBeginPlay`)
  (set `self.OrgLoc` (`SceneComponent.K2_GetComponentLocation` (`self.KillBox`))) ; For resetting position
)

(event `self.OnTrapTrigger`
  (params (Player :type "/Game/Blueprints/Characters/BP_RageCharacter Object Reference"))
  (bind _state (`self.GetTriggerComponentActive` (`self.TriggerBox`)))
  (if _state
    (`parent.OnTrapTrigger` Player)
    (bind (_direction _dropval) (`Timeline|CeilingDrop` :!via `PlayFromStart` :!label _label)
      (:`Update`
        (`SceneComponent.K2_SetWorldLocation` (`self.KillBox`) (+ (`self.OrgLoc`) (* (`KismetMathLibrary.Vector_Down`) (* (`self.Distance`) (* (`self.Speed`) _dropval)))) false false))
      (:`Finished`
        (if (not (`self.TrapReady`))
          (`parent.OnTrapReset`))))))

(event `self.OnTrapReset`
  (goto _label :!via `ReverseFromEnd`))

(event `self.OnKill`
  (params (Player :type "/Game/Blueprints/Characters/BP_RageCharacter Object Reference"))
  (`KismetSystemLibrary.PrintString` "Crushed")
  (`parent.OnKill` Player))

(fn `UserConstructionScript`
  (`parent.UserConstructionScript`))