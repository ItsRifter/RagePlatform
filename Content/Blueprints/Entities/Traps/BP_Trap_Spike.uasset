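; Spike trap Blueprint that builds on a parent trap class, raising spikes when triggered and lowering them on reset.
; The spike mesh starts hidden in its down montage, becomes visible with the up montage on trigger, and returns to hidden on reset.
; On a kill, it passes a random death text to the RGameInstance before running the parent kill logic.
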(event `self.ReceiveBeginPlay`
  (`parent.ReceiveBeginPlay`)
  (`SceneComponent.SetVisibility` (`self.M_Spikes`) false true)
  (`|PlayMontage` (`self.M_Spikes`) "/Game/Animation_Import/Spikes/Assets/Spike_M_Down.Spike_M_Down"))

(event `self.OnTrapTrigger`
  (params (Player :type "/Game/Blueprints/Characters/BP_RageCharacter Object Reference"))
  (if true
    (`parent.OnTrapTrigger` Player)
    (`SceneComponent.SetVisibility` (`self.M_Spikes`) true true)
    (`|PlayMontage` (`self.M_Spikes`) "/Game/Animation_Import/Spikes/Assets/Spike_M_Up.Spike_M_Up")))

(event `self.OnTrapReset`
  (`parent.OnTrapReset`)
  (`SceneComponent.SetVisibility` (`self.M_Spikes`) false true)
  (`|PlayMontage` (`self.M_Spikes`) "/Game/Animation_Import/Spikes/Assets/Spike_M_Down.Spike_M_Down"))

(event `self.OnKill`
  (params (Player :type "/Game/Blueprints/Characters/BP_RageCharacter Object Reference"))
  (`KismetSystemLibrary.PrintString` "Spiked")
  (bind _asrgame_instance (cast `RGameInstance` (`GameplayStatics.GetGameInstance`)))
  (`RGameInstance.SetOnPlayerDeath` _asrgame_instance (`|GetArrayItem` (`self.Death Text`) (`KismetMathLibrary.RandomInteger` (`self.Exclusive Max`))))
  (`parent.OnKill` Player))

(fn `UserConstructionScript`)