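; Base Blueprint for traps, with a trigger box that fires the trap and a kill box that kills BP_RageCharacter on overlap.
; Triggering calls OnTrapTrigger, clears TrapReady and starts a ResetTime timer that re-arms it via OnTrapReset.
; Each box checks its active state and disable flag before acting.
; BeginPlay activates both boxes, or prints a red warning instead if both are disabled.
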(event `self.ReceiveBeginPlay`
  (if (and (`self.DisableTrigger`) (`self.DisableKillBox`))
    (`KismetSystemLibrary.PrintString` (`KismetStringLibrary.Concat_StrStr` (`KismetSystemLibrary.GetDisplayName` self) " has both trigger and kill boxes disabled") true true (struct :`R` 1.0 :`A` 1.0) 3.0)
    (else
      (`ActorComponent.SetActive` (`self.KillBox`) true false)
      (`ActorComponent.SetActive` (`self.TriggerBox`) true false))))

(event `OnKill`
  (params (Player :type "/Game/Blueprints/Characters/BP_RageCharacter Object Reference"))
  (if (`ActorComponent.IsActive` (`self.KillBox`))
    (`RageCharacter.Death` Player)))

(event `OnTrapTrigger`
  (params (Player :type "/Game/Blueprints/Characters/BP_RageCharacter Object Reference"))
  (set `self.TrapReady` false))

(event `self.TriggerBox.OnComponentBeginOverlap`
  (params (OverlappedComponent :type "PrimitiveComponent Object Reference") (OtherActor :type "Actor Object Reference") (OtherComp :type "PrimitiveComponent Object Reference") (OtherBodyIndex :type Integer) (bFromSweep :type Boolean) (SweepResult :type "HitResult Structure (by ref)"))
  (bind _state (`self.GetTriggerComponentActive` (`self.TriggerBox`)))
  (if _state
    (if (and (`self.TrapReady`) (not (`self.DisableTrigger`)))
      (bind _asbp_rage_character (cast `/Game/Blueprints/Characters/BP_RageCharacter` OtherActor))
      (`self.OnTrapTrigger` _asbp_rage_character)
      (bind _returnvalue (`KismetSystemLibrary.K2_SetTimerDelegate` (delegate `OnTrapReset`) (`self.ResetTime`)))
      (set `self.ResetTimerHandle` _returnvalue)
      (set `self.TrapReady` false))))

(event `OnTrapReset`
  (set `self.TrapReady` true))

(event `self.KillBox.OnComponentBeginOverlap`
  (params (OverlappedComponent :type "PrimitiveComponent Object Reference") (OtherActor :type "Actor Object Reference") (OtherComp :type "PrimitiveComponent Object Reference") (OtherBodyIndex :type Integer) (bFromSweep :type Boolean) (SweepResult :type "HitResult Structure (by ref)"))
  (bind _state (`self.GetTriggerComponentActive` (`self.KillBox`)))
  (if _state
    (if (not (`self.DisableKillBox`))
      (bind _asbp_rage_character (cast `/Game/Blueprints/Characters/BP_RageCharacter` OtherActor))
      (`self.OnKill` _asbp_rage_character))))

(fn `GetTriggerComponentActive`
  (params (Component :type "ActorComponent Object Reference"))
  (returns (State :type Boolean))
  (return (`ActorComponent.IsActive` Component)))

(fn `UserConstructionScript`)