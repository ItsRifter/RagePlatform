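; Base trap actor that activates when BP_RageCharacter enters its trigger box and kills that character on contact with its kill box.
; Triggering plays an activation sound and blocks retriggering until a reset timer re-arms it; kills call Death and play a 2D sound.
; Either box can be disabled, and BeginPlay prints a warning if both are.
; A helper event attaches an optional loop sound, while the game-instance death-message calls are left unconnected.
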(event `SetupLoopSound`
  (params (Component :type "SceneComponent Object Reference"))
  (bind _loopsound (`self.LoopSound`)
    (:`then`
      (`GameplayStatics.SpawnSoundAttached` _loopsound Component "None" (0.0 0.0 0.0) (struct) "KeepRelativeOffset" false 1.0 1.0 0.0 "/Game/Sounds/SA_Trap.SA_Trap" null))
    (:`else`)))

(event `self.ReceiveBeginPlay`
  (if (and (`self.DisableTrigger`) (`self.DisableKillBox`))
    (`KismetSystemLibrary.PrintString` (`KismetStringLibrary.Concat_StrStr` (`KismetSystemLibrary.GetDisplayName` self) " has both trigger and kill boxes disabled") true true (struct :`R` 1.0 :`A` 1.0) 3.0) ; Warn that this trap is setup incorrectly
    (else
      (`ActorComponent.SetActive` (`self.KillBox`) true false)
      (`ActorComponent.SetActive` (`self.TriggerBox`) true false)
      (bind _asrgame_instance (cast `RGameInstance` (`GameplayStatics.GetGameInstance`))))))

(event `OnTrapTrigger`
  (params (Player :type "/Game/Blueprints/Characters/BP_RageCharacter Object Reference"))
  (bind _audio (`self.Audio`))
  ;[0.01757 0.8031 0.7479 0.5] Trap trigger
  (set `self.TrapReady` false)
  (bind _activatesound (`self.ActivateSound`)
    (:`then`
      (`AudioComponent.SetSound` _audio _activatesound)
      (`AudioComponent.Play` _audio 0.0))
    (:`else`)))

(event `OnKill`
  (params (Player :type "/Game/Blueprints/Characters/BP_RageCharacter Object Reference"))
  ;[0.874 0.01875 0 0.5] Player killed by trap
  (`RageCharacter.Death` Player)
  (bind _killsound (`self.KillSound`)
    (:`then`
      (`GameplayStatics.SpawnSound2D` _killsound 1.0 1.0 0.0 null))
    (:`else`)))

(event `self.TriggerBox.OnComponentBeginOverlap`
  (params (OverlappedComponent :type "PrimitiveComponent Object Reference") (OtherActor :type "Actor Object Reference") (OtherComp :type "PrimitiveComponent Object Reference") (OtherBodyIndex :type Integer) (bFromSweep :type Boolean) (SweepResult :type "HitResult Structure (by ref)"))
  ;[0 0.5381 1 0.5] Triggerbox activated by player - Handles trap activation
  (bind _state (`self.GetTriggerComponentActive` (`self.TriggerBox`)))
  (if _state
    (if (and (`self.TrapReady`) (not (`self.DisableTrigger`)))
      (bind _asbp_rage_character (cast `/Game/Blueprints/Characters/BP_RageCharacter` OtherActor))
      (`self.OnTrapTrigger` _asbp_rage_character)
      (bind _returnvalue (`KismetSystemLibrary.K2_SetTimerDelegate` (delegate `OnTrapReset`) (`self.ResetTime`)))
      (set `self.ResetTimerHandle` _returnvalue)
      (set `self.TrapReady` false))))

(event `OnTrapReset`
  ;[0 0.5381 1 0.5] Triggerbox activated by player - Handles trap activation
  (set `self.TrapReady` true))

(event `self.KillBox.OnComponentBeginOverlap`
  (params (OverlappedComponent :type "PrimitiveComponent Object Reference") (OtherActor :type "Actor Object Reference") (OtherComp :type "PrimitiveComponent Object Reference") (OtherBodyIndex :type Integer) (bFromSweep :type Boolean) (SweepResult :type "HitResult Structure (by ref)"))
  ;[0.1615 0 5.9e-05 0.5] Killbox activated by player - Handles killing the player
  (bind _state (`self.GetTriggerComponentActive` (`self.KillBox`)))
  (if _state
    (if (and (not (`self.DisableKillBox`)) (`ActorComponent.IsActive` (`self.KillBox`)))
      (bind _asbp_rage_character (cast `/Game/Blueprints/Characters/BP_RageCharacter` OtherActor))
      (`self.OnKill` _asbp_rage_character))))

(fn `GetTriggerComponentActive`
  (params (Component :type "ActorComponent Object Reference"))
  (returns (State :type Boolean))
  (return (`ActorComponent.IsActive` Component)))

(fn `UserConstructionScript`)