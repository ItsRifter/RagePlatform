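; Rotor sawblade trap that shuttles back and forth along its pivot's forward axis with a looping sound.
; A timeline offsets the pivot from the blade's starting location and spins the blade, reversing each time it finishes.
; Each reversal also tells the Saw_ABP animation blueprint to switch direction.
; On kill, it prints a debug string and passes death text to RGameInstance before calling the parent's kill logic.
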(event `self.ReceiveBeginPlay`
  (`parent.ReceiveBeginPlay`)
  (set `self.OrgLoc` (`SceneComponent.K2_GetComponentLocation` (`self.Sawblade_Anim_Spin`)))
  (`self.DoRotorForward`)
  (`self.SetupLoopSound` (`self.Pivot`)))

(event `DoRotorForward`
  (set `self.IsMovingBack` false)
  (bind _assaw_abp (cast `/Game/Animation_Import/Sawblade/Assets/Saw_ABP` (`SkeletalMeshComponent.GetAnimInstance` (`self.Sawblade_Anim_Spin`))))
  (`/Game/Animation_Import/Sawblade/Assets/Saw_ABP.SwitchDirection` _assaw_abp)
  (bind (_direction _spinval) (`Timeline|MoveTimeline` :!label _label)
    (:`Update`
      (`SceneComponent.K2_SetWorldLocation` (`self.Pivot`) (+ (`self.OrgLoc`) (* (`SceneComponent.GetForwardVector` (`self.Pivot`)) (* (`self.Dist`) _spinval))) false false)
      (`SceneComponent.K2_AddLocalRotation` (`self.Sawblade_Anim_Spin`) (`KismetMathLibrary.MakeRotator` 0.0 (`self.RotorSpeed`)) false false))
    (:`Finished`
      (if (`self.IsMovingBack`)
        (`self.DoRotorForward`)
        (else
          (`self.DoRotorBackward`))))))

(event `DoRotorBackward`
  (set `self.IsMovingBack` true)
  (bind _assaw_abp (cast `/Game/Animation_Import/Sawblade/Assets/Saw_ABP` (`SkeletalMeshComponent.GetAnimInstance` (`self.Sawblade_Anim_Spin`))))
  (`/Game/Animation_Import/Sawblade/Assets/Saw_ABP.SwitchDirection` _assaw_abp)
  (goto _label :!via `Reverse`))

(event `self.OnKill`
  (params (Player :type "/Game/Blueprints/Characters/BP_RageCharacter Object Reference"))
  (`KismetSystemLibrary.PrintString` "Sawed")
  (bind _asrgame_instance (cast `RGameInstance` (`GameplayStatics.GetGameInstance`)))
  (`RGameInstance.SetOnPlayerDeath` _asrgame_instance (`self.Death Text`))
  (`parent.OnKill` Player))

(fn `UserConstructionScript`
  (`parent.UserConstructionScript`))