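; Pooled trap arrow projectile that kills the rage character on contact.
; SetInUse extends the parent logic, launching the projectile along the ArrowTrap forward vector or zeroing its velocity when released.
; A KillBox overlap with the character triggers PlayerFall with a directional push, passes death text to the game instance and releases the arrow.
; Other actors tagged ParticleCollide also release it.
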(event `self.SetInUse`
  (params (SetUse :type Boolean) (Lifetime :type "Float (double-precision)"))
  (`parent.SetInUse` SetUse Lifetime)
  (if SetUse
    (set `MovementComponent.Velocity` (* (`SceneComponent.GetForwardVector` (`self.Arrow_Trap`)) 700.0) (`self.ProjectileMovement`))
    (else
      (set `MovementComponent.Velocity` (0.0 0.0 0.0) (`self.ProjectileMovement`)))))

(event `self.KillBox.OnComponentBeginOverlap`
  (params (OverlappedComponent :type "PrimitiveComponent Object Reference") (OtherActor :type "Actor Object Reference") (OtherComp :type "PrimitiveComponent Object Reference") (OtherBodyIndex :type Integer) (bFromSweep :type Boolean) (SweepResult :type "HitResult Structure (by ref)"))
  (bind _asbp_rage_character (cast `/Game/Blueprints/Characters/BP_RageCharacter` OtherActor)
    (:`then`
      (`RageCharacter.PlayerFall` _asbp_rage_character (* (`KismetMathLibrary.GetForwardVector` (`SceneComponent.K2_GetComponentRotation` (`self.Arrow_Trap2`))) 350.0))
      (bind _asrgame_instance (cast `RGameInstance` (`GameplayStatics.GetGameInstance`)))
      (`RGameInstance.SetOnPlayerDeath` _asrgame_instance (`self.Death Text`))
      (`self.SetInUse` false))
    (:`CastFailed`
      (if (`self.ActorHasTag` OtherActor "ParticleCollide")
        (`self.SetInUse` false)))))

(fn `UserConstructionScript`)