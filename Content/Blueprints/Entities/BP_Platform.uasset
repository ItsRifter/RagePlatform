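; BP_Platform is a moving platform actor that reacts to path markers it travels through.
; When its Box overlaps a BP_PlatformPath listed in its PlatformComponent's Paths, it notifies that path through OnPass.
; It then sets the move component's speed multiplier from that path's MoveMultiplier, so each path point can change the platform's speed.
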(event `self.Box.OnComponentBeginOverlap`
  (params (OverlappedComponent :type "PrimitiveComponent Object Reference") (OtherActor :type "Actor Object Reference") (OtherComp :type "PrimitiveComponent Object Reference") (OtherBodyIndex :type Integer) (bFromSweep :type Boolean) (SweepResult :type "HitResult Structure (by ref)"))
  (bind _asbp_platform_path (cast `/Game/Blueprints/Entities/BP_PlatformPath` OtherActor))
  (if (!= (`KismetArrayLibrary.Array_Find` (`PlatformComponent.Paths` (`self.PlatformComponent`)) _asbp_platform_path) -1)
    (`PlatformPath.OnPass` _asbp_platform_path)
    (set `InterpToMovementComponent.SpeedMultiplier` (`PlatformPath.MoveMultiplier` _asbp_platform_path) (`PlatformComponent.MoveComponent` (`self.PlatformComponent`)))))

(fn `UserConstructionScript`)