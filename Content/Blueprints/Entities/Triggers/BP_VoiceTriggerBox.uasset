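; BP_VoiceTriggerBox is a trigger box that plays a sequence of voicelines when BP_RageCharacter overlaps it.
; PlayVoicelines re-calls itself after each clip's duration plus a short gap, then destroys the actor after the last.
; An IsPlaying flag blocks repeat triggers.
; The player's skip-dialogue request stops the audio and clears that flag, without cancelling the pending delay.
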(event `self.ReceiveBeginPlay`
  (bind _asbp_rage_character (cast `/Game/Blueprints/Characters/BP_RageCharacter` (`GameplayStatics.GetPlayerCharacter` 0)))
  (add `/Game/Blueprints/Characters/BP_RageCharacter.RequestSkipDialogue` _asbp_rage_character (delegate `ForceSkip`)))

(event `ForceSkip`
  ; Skip dialogue
  (`AudioComponent.Stop` (`self.Audio`))
  (set `self.IsPlaying` false))

(event `PlayVoicelines`
  (bind _audio (`self.Audio`))
  (bind _voicelines (`self.Voicelines`))
  (bind _voiceindex (`self.VoiceIndex`))
  (bind _output (`|GetArrayItem` _voicelines _voiceindex))
  ;[0.1734 0.6698 0.01905 0.5] Plays voicelines in sequential order
  (if (== (`KismetArrayLibrary.Array_Length` _voicelines) _voiceindex)
    (`self.K2_DestroyActor`)
    (else
      (`AudioComponent.SetSound` _audio _output)
      (`AudioComponent.Play` _audio 0.0)
      (`KismetSystemLibrary.Delay` (+ (`SoundBase.Duration` _output) 0.4))
      (`/Engine/EditorBlueprintResources/StandardMacros.IncrementInt` (`self.VoiceIndex`)
        (:`  `
          (`self.PlayVoicelines`))))))

(event `self.Box.OnComponentBeginOverlap`
  (params (OverlappedComponent :type "PrimitiveComponent Object Reference") (OtherActor :type "Actor Object Reference") (OtherComp :type "PrimitiveComponent Object Reference") (OtherBodyIndex :type Integer) (bFromSweep :type Boolean) (SweepResult :type "HitResult Structure (by ref)"))
  ; Trigger event
  (cast `/Game/Blueprints/Characters/BP_RageCharacter` OtherActor)
  (if (not (`self.IsPlaying`))
    (`self.PlayVoicelines`)
    (set `self.IsPlaying` true)))

(fn `UserConstructionScript`)