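; Level change actor that records the player's stats in RGameInstance when its CompletedLevel event fires.
; The event refreshes name, death count and game time in PlayerStats, then adds a LevelTime entry keyed by level number only if none exists.
; That entry uses the passed player time, or the instance's TimeVar when game time is zero, formatted by ConvertToTime as minutes:seconds:hundredths.
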(event `self.CompletedLevel`
  (params (PlayerTime :type "Float (single-precision)") (GameTime :type "Float (single-precision)"))
  ;[0 0 0] Handling Storing Player Stats
  (bind _asrgame_instance (cast `RGameInstance` (`GameplayStatics.GetGameInstance`)))
  (bind _convertedtimeformat (`self.ConvertToTime` PlayerTime))
  (bind (_playerstats_playername _playerstats_leveltime) (break `PlayerStats` (`RGameInstance.PlayerStats` _asrgame_instance)))
  (set `RGameInstance.PlayerStats` (make `PlayerStats` (`KismetTextLibrary.Conv_TextToString` (`RGameInstance.PlayerName` _asrgame_instance)) _playerstats_leveltime (`KismetStringLibrary.Conv_IntToString` (`RGameInstance.DeathCount` _asrgame_instance)) GameTime) _asrgame_instance)
  (bind _levelnumber (`RGameInstance.LevelNumber` _asrgame_instance))
  (if (`BlueprintMapLibrary.Map_Contains` _playerstats_leveltime _levelnumber)
    _
    (elif (== GameTime 0.0)
      (bind _convertedtimeformat_2 (`self.ConvertToTime` (`RGameInstance.TimeVar` _asrgame_instance)))
      (`BlueprintMapLibrary.Map_Add` _playerstats_leveltime _levelnumber _convertedtimeformat_2)
      (else
        (`BlueprintMapLibrary.Map_Add` _playerstats_leveltime _levelnumber _convertedtimeformat)))))

(fn `ConvertToTime`
  (params (TimeFloat :type "Float (double-precision)"))
  (returns (ConvertedTimeFormat :type String))
  (bind _returnvalue (`KismetMathLibrary.FFloor` TimeFloat))
  (return (`KismetStringLibrary.Concat_StrStr` (`KismetStringLibrary.Conv_IntToString` (/ (mod _returnvalue 3600) 60)) ":" (`KismetStringLibrary.Conv_IntToString` (mod _returnvalue 60)) ":" (`KismetStringLibrary.Conv_IntToString` (`KismetMathLibrary.Round` (* (- TimeFloat _returnvalue) 100.0))))))

(fn `UserConstructionScript`)