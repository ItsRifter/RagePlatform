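; BP_TrapShooter_Base is a base trap that repeatedly fires pooled projectile particles from its Arrow component.
; BeginPlay sets a one-shot startup timer and also starts the looping fire timer, which StartupWait sets again once the delay elapses.
; Each shot spawns from the ObjectPool at the Arrow's location and rotation with a set lifetime, takes the trap as owner and plays the fire sound.
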(event `self.ReceiveBeginPlay`
  (`KismetSystemLibrary.K2_SetTimerDelegate` (delegate `StartupWait`) (`self.TimeDelay`)) ; Delay first shooting
  (bind _returnvalue (`KismetSystemLibrary.K2_SetTimerDelegate` (delegate `FireParticle`) (`self.TimeToShoot`) true :!label _label))
  (set `self.ShootTimer` _returnvalue))

(event `FireParticle`
  (bind _audio (`self.Audio`))
  (bind _poolactor (`/Game/Blueprints/Misc/AC_ObjectPool.SpawnFromPool` (`self.ObjectPool`) (`KismetMathLibrary.MakeTransform` (`SceneComponent.K2_GetComponentLocation` (`self.Arrow`)) (`SceneComponent.K2_GetComponentRotation` (`self.Arrow`))) (`self.ParticleLifetime`)))
  (`self.SetOwner` _poolactor self)
  (`AudioComponent.SetSound` _audio "/Game/Sounds/Traps/Shooter/MS_ShooterFire.MS_ShooterFire")
  (`AudioComponent.Play` _audio 0.0))

(event `StartupWait`
  (goto _label))

(fn `UserConstructionScript`)