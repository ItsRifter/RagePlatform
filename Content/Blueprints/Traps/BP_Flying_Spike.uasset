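; BP_Flying_Spike is a trap that launches a spike as a projectile when triggered.
; OnTrapTrigger saves the mesh's world location, calls the parent trigger, then sets projectile velocity along the Direction component's forward vector, scaled by Test.
; The KillBox overlap only casts to BP_RageCharacter.
; Death reporting to RGameInstance and the reset to the saved location are disconnected and never run.
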(event `self.OnTrapTrigger`
  (params (Player :type "/Game/Blueprints/Characters/BP_RageCharacter Object Reference"))
  (set `self.Location` (`SceneComponent.K2_GetComponentLocation` (`self.SkeletalMesh`)))
  (if true
    (`parent.OnTrapTrigger` Player)
    (set `MovementComponent.Velocity` (* (`SceneComponent.GetForwardVector` (`self.Direction`)) (`self.Test`)) (`self.ProjectileMovement`))
    (else
      (set `MovementComponent.Velocity` (0.0 0.0 0.0) (`self.ProjectileMovement`)))))

(event `self.KillBox.OnComponentBeginOverlap`
  (params (OverlappedComponent :type "PrimitiveComponent Object Reference") (OtherActor :type "Actor Object Reference") (OtherComp :type "PrimitiveComponent Object Reference") (OtherBodyIndex :type Integer) (bFromSweep :type Boolean) (SweepResult :type "HitResult Structure (by ref)"))
  (cast `/Game/Blueprints/Characters/BP_RageCharacter` OtherActor))

(fn `UserConstructionScript`)