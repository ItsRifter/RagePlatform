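; Explosive trap Blueprint whose scorch mark becomes more opaque as player kills accumulate.
; On BeginPlay it creates a dynamic scorch material on the decal component and applies the starting opacity.
; Each OnPlayerKill event raises the stored opacity by a fixed step up to a cap and updates the material parameter.
; The DecalVisible event syncs the scorch component's visibility to that of the static mesh.
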(event `self.DecalVisible`
  (`self. VisibileMesh`))

(event `self.ReceiveBeginPlay`
  (bind _returnvalue (`PrimitiveComponent.CreateDynamicMaterialInstance` (`self.Explosion_Decal_Export_Shorter`) 0 "/Game/Materials/Decals/Explosion_Scorch_3.Explosion_Scorch_3" "None"))
  (bind _output_get (set `self.MatInstance` _returnvalue))
  (`MaterialInstanceDynamic.SetScalarParameterValue` _output_get "OpacityParam" (`self.Opacity`)))

(event `self.OnPlayerKill`
  (bind _output_get (set `self.Opacity` (`KismetMathLibrary.FClamp` (+ (`self.Opacity`) 0.2666) 0.0 0.8)))
  (`MaterialInstanceDynamic.SetScalarParameterValue` (`self.MatInstance`) "OpacityParam" _output_get))

(fn ` VisibileMesh`
  (bind _output_get (set `self.StaticMeshVisible?` (`SceneComponent.IsVisible` (`self.StaticMesh`))))
  (if _output_get
    (`SceneComponent.SetVisibility` (`self.Explosion_Decal_Export_Shorter`) true false)
    (else
      (`SceneComponent.SetVisibility` (`self.Explosion_Decal_Export_Shorter`) false false))))

(fn `UserConstructionScript`)