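; Arrow trap projectile that kills the player on contact, built on a parent's in-use toggle with a lifetime.
; Entering use launches it along the arrow mesh's forward vector; leaving use zeroes its velocity.
; KillBox overlaps with a living BP_RageCharacter trigger a knockback fall, camera focus on the owner, death text and death.
; Overlaps with actors or components tagged ParticleCollide play an impact sound and, like player hits, release the arrow.
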(event `self.SetInUse`
  (params (SetUse :type Boolean) (Lifetime :type "Float (double-precision)"))
  (`parent.SetInUse` SetUse Lifetime)
  (if SetUse
    (set `MovementComponent.Velocity` (* (`SceneComponent.GetForwardVector` (`self.Arrow_Trap`)) 700.0) (`self.ProjectileMovement`))
    (else
      (set `MovementComponent.Velocity` (0.0 0.0 0.0) (`self.ProjectileMovement`)))))

(event `self.KillBox.OnComponentBeginOverlap`
  (params (OverlappedComponent :type "PrimitiveComponent Object Reference") (OtherActor :type "Actor Object Reference") (OtherComp :type "PrimitiveComponent Object Reference") (OtherBodyIndex :type Integer) (bFromSweep :type Boolean) (SweepResult :type "HitResult Structure (by ref)"))
  (bind _asbp_rage_character (cast `/Game/Blueprints/Characters/BP_RageCharacter` OtherActor)
    (:`then`
      (`RageCharacter.bIsAlive` _asbp_rage_character
        (:`then`
          (`RageCharacter.PlayerFall` _asbp_rage_character (* (`KismetMathLibrary.GetForwardVector` (`SceneComponent.K2_GetComponentRotation` (`self.Arrow_Trap2`))) 200.0))
          (bind _temp_camera (`RageCharacter.Temp_Camera` _asbp_rage_character))
          (set `RTempCamera.FocusVar` (`self.GetOwner`) _temp_camera)
          (`RTempCamera.StartFocus` _temp_camera)
          (bind _asrgame_instance (cast `RGameInstance` (`GameplayStatics.GetGameInstance`)))
          (`RGameInstance.SetOnPlayerDeath` _asrgame_instance (`self.Death Text`))
          (`RageCharacter.OnDeath` _asbp_rage_character "Arrows")
          (`self.SetInUse` false)
          (`GameplayStatics.PlaySound2D` "/Game/Sounds/Traps/Shooter/MS_ArrowHit_Body.MS_ArrowHit_Body" 1.0 1.0 0.0 null null))
        (:`else`)))
    (:`CastFailed`
      (if (`self.ActorHasTag` OtherActor "ParticleCollide")
        (`GameplayStatics.PlaySoundAtLocation` "/Game/Sounds/Traps/Shooter/MS_ArrowHit.MS_ArrowHit" (`SceneComponent.K2_GetComponentLocation` (`self.DefaultSceneRoot`)) (struct) 1.0 1.0 0.0 "/Game/Sounds/SA_Trap_Short.SA_Trap_Short" null null null :!label _label)
        (`self.SetInUse` false)
        (elif (`ActorComponent.ComponentHasTag` OtherComp "ParticleCollide")
          (goto _label))))))

(fn `UserConstructionScript`)