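; BP_TempCam is a camera actor, stored with trap test assets, that smoothly turns its camera toward a point slightly above an actor location.
; Each Tick, after a validity check, it interpolates the camera's world rotation toward a look-at rotation using RInterpTo.
; StartFocus and StopFocus are empty, and the nodes for enabling and disabling actor tick are disconnected, so neither event controls the tracking.
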(event `StartFocus`)

(event `StopFocus`)

(event `self.ReceiveTick`
  (params (DeltaSeconds :type "Float (single-precision)"))
  (bind _camera (`self.Camera`))
  (`/Engine/EditorBlueprintResources/StandardMacros.IsValid` null
    (:`Is Valid`
      (`SceneComponent.K2_SetWorldRotation` (`self.Camera`) (`KismetMathLibrary.RInterpTo` (`SceneComponent.K2_GetComponentRotation` _camera) (`KismetMathLibrary.FindLookAtRotation` (`SceneComponent.K2_GetComponentLocation` _camera) (+ (`self.K2_GetActorLocation`) (0.0 0.0 50.0))) (`GameplayStatics.GetWorldDeltaSeconds`) 3.0) false false))))

(fn `UserConstructionScript`)