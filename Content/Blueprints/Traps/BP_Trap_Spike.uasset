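; Spike trap Blueprint built on a parent trap class, driving a spike skeletal mesh through the trap lifecycle.
; Spikes start hidden in the down montage, become visible with the up montage when triggered, and return to hidden and down on reset.
; On a kill, it prints a debug string and passes death text to RGameInstance before deferring to the parent kill logic, which is skipped if that cast fails.
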(event `self.ReceiveBeginPlay`
  (bind _m_spikes (`self.M_Spikes`))
  (`parent.ReceiveBeginPlay`)
  (`SceneComponent.SetVisibility` _m_spikes false false)
  (`|PlayMontage` _m_spikes "/Game/Blueprints/Animation/Spikes/Spike_M_Down.Spike_M_Down"))

(event `self.OnTrapTrigger`
  (params (Player :type "/Game/Blueprints/Characters/BP_RageCharacter Object Reference"))
  (bind _m_spikes (`self.M_Spikes`))
  (if true
    (`parent.OnTrapTrigger` Player)
    (`SceneComponent.SetVisibility` _m_spikes true false)
    (`|PlayMontage` _m_spikes "/Game/Blueprints/Animation/Spikes/Spike_M_Up.Spike_M_Up")))

(event `self.OnTrapReset`
  (bind _m_spikes (`self.M_Spikes`))
  (`parent.OnTrapReset`)
  (`SceneComponent.SetVisibility` _m_spikes false false)
  (`|PlayMontage` _m_spikes "/Game/Blueprints/Animation/Spikes/Spike_M_Down.Spike_M_Down"))

(event `self.OnKill`
  (params (Player :type "/Game/Blueprints/Characters/BP_RageCharacter Object Reference"))
  (`KismetSystemLibrary.PrintString` "Spiked")
  (bind _asrgame_instance (cast `RGameInstance` (`GameplayStatics.GetGameInstance`)))
  (`RGameInstance.SetOnPlayerDeath` _asrgame_instance (`self.Death Text`))
  (`parent.OnKill` Player))

(fn `UserConstructionScript`)