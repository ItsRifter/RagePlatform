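; Wall spike trap that fires either when triggered or on a looping random timer, building on a parent trap's begin-play, trigger and kill logic.
; A firing plays a sound, shows the placeholder arrow mesh and enables collision, then reverses the sliding timeline after a hold delay.
; Loop mode ignores triggers, disabling collision and re-arming between a clamped min and max time.
; Trap reset re-readies only non-looping traps.
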(event `SpikeIn`
  (set `self.IsActive` true)
  (`self.SetActorEnableCollision` true)
  (`SceneComponent.SetVisibility` (`self.ArrowPlaceholder`) false false)
  (bind (_direction _dist) (`Timeline|InOut` :!via `PlayFromStart` :!label _label)
    (:`Update`
      (`SceneComponent.K2_SetRelativeLocation` (`self.ArrowPlaceholder`) (* (`SceneComponent.GetForwardVector` (`self.ArrowPlaceholder`)) (* (`self.InactiveOffset`) _dist)) false false))
    (:`Finished`
      (if (not (`self.IsActive`))
        (`SceneComponent.SetVisibility` (`self.ArrowPlaceholder`) false false)
        (`self.DoActivateSound`)))))

(event `SpikeOut`
  (set `self.IsActive` false)
  (goto _label :!via `ReverseFromEnd`))

(event `DoActivateSound`
  (bind _audio (`self.Audio`))
  (bind _activatesound (`self.ActivateSound`)
    (:`then`
      (`AudioComponent.SetSound` _audio _activatesound)
      (`AudioComponent.Play` _audio 0.0))
    (:`else`)))

(event `self.ReceiveBeginPlay`
  (bind _arrowplaceholder (`self.ArrowPlaceholder`))
  ; Beginplay - MinMax check + OnLoopTimer
  (`SceneComponent.K2_SetRelativeLocation` _arrowplaceholder (* (`SceneComponent.GetForwardVector` _arrowplaceholder) (`self.InactiveOffset`)) false false)
  (`parent.ReceiveBeginPlay`)
  (set `self.MaxLoopTime` (`KismetMathLibrary.FMax` (`self.MinLoopTime`) (`self.MaxLoopTime`))) ; If min exceeds max, set as max
  (if (`self.OnLoopTimer`)
    (`self.SetActorEnableCollision` false)
    (`SceneComponent.SetVisibility` (`self.ArrowPlaceholder`) false false)
    (`self.ResetTimer`)
    (else
      (`SceneComponent.SetVisibility` (`self.ArrowPlaceholder`) false false))))

(event `ResetTimer`
  ; Resets Timer with random time
  (`self.SetActorEnableCollision` false)
  (bind _returnvalue (`KismetSystemLibrary.K2_SetTimerDelegate` (delegate `DoWallSpike`) (`KismetMathLibrary.RandomFloatInRange` (`self.MinLoopTime`) (`self.MaxLoopTime`))))
  (set `self.TimerHandle` _returnvalue))

(event `self.OnTrapTrigger`
  (params (Player :type "/Game/Blueprints/Characters/BP_RageCharacter Object Reference"))
  (if true
    (if (not (`self.OnLoopTimer`))
      (`parent.OnTrapTrigger` Player)
      (`self.DoWallSpike`))))

(event `self.OnKill`
  (params (Player :type "/Game/Blueprints/Characters/BP_RageCharacter Object Reference"))
  (`parent.OnKill` Player))

(event `DoWallSpike`
  ; Trap Activation
  (if (`self.OnLoopTimer`)
    (`KismetSystemLibrary.K2_ClearAndInvalidateTimerHandle` (`self.TimerHandle`)))
  (`self.SpikeIn`)
  (`self.DoActivateSound`)
  (`SceneComponent.SetVisibility` (`self.ArrowPlaceholder`) true false)
  (`KismetSystemLibrary.Delay` (`self.HoldTime`))
  (`self.SpikeOut`)
  (if (`self.OnLoopTimer`)
    (`self.ResetTimer`)))

(event `self.OnTrapReset`
  (if (not (`self.OnLoopTimer`))
    (set `self.TrapReady` true)))

(fn `UserConstructionScript`
  (`parent.UserConstructionScript`))