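; BP_Trap_Dummy is a placeholder trap in the OLD traps folder that only reports its events through debug text.
; Its trigger, reset and kill events each print the actor's display name with a status word or phrase.
; It contains no trap behavior of its own, and its construction script is empty.
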(event `self.OnTrapTrigger`
  (params (Player :type "/Game/Blueprints/Characters/BP_RageCharacter Object Reference"))
  (`KismetSystemLibrary.PrintString` (`KismetStringLibrary.Concat_StrStr` (`KismetSystemLibrary.GetDisplayName` self) " Activated")))

(event `self.OnTrapReset`
  (`KismetSystemLibrary.PrintString` (`KismetStringLibrary.Concat_StrStr` (`KismetSystemLibrary.GetDisplayName` self) " Reset")))

(event `self.OnKill`
  (params (Player :type "/Game/Blueprints/Characters/BP_RageCharacter Object Reference"))
  (`KismetSystemLibrary.PrintString` (`KismetStringLibrary.Concat_StrStr` (`KismetSystemLibrary.GetDisplayName` self) " Killed the player")))

(fn `UserConstructionScript`)