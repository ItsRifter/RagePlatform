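; Actor component that provides an object pool, reusing pre-spawned actors of a configurable class instead of spawning new ones on demand.
; On BeginPlay it spawns the pool and marks every actor as not in use.
; SpawnFromPool linearly searches for the first free actor, moves it to the given transform and activates it with a lifetime.
; The pool never grows, so no actor is returned when all are busy.
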(event `self.ReceiveBeginPlay`
  (`self.InitializePool`))

(event `InitializePool`
  (for _ (range (+ (`self.PoolSize`) 1))
    (bind _returnvalue (`|SpawnActorFromClass` (`self.PooledActorClass`) (`KismetMathLibrary.MakeTransform` (0.0 0.0 0.0)) "Undefined" "MultiplyWithRoot" null null))
    (`KismetArrayLibrary.Array_AddUnique` (`self.ObjectPool`) _returnvalue)
    (`/Game/Blueprints/Misc/BP_PoolActor.SetInUse` _returnvalue false 1.0)))

(fn `FindFirstAvailable`
  (returns (Found :type "/Game/Blueprints/Misc/BP_PoolActor Object Reference"))
  (for _array_element (`self.ObjectPool`)
    (if (not (`/Game/Blueprints/Misc/BP_PoolActor.InUse` _array_element))
      (return _array_element))))

(fn `SpawnFromPool`
  (params (SpawnTransform :type "Transform Structure") (Lifetime :type "Float (double-precision)" :default 1.0))
  (returns (PoolActor :type "/Game/Blueprints/Misc/BP_PoolActor Object Reference"))
  (bind _found (`self.FindFirstAvailable`))
  (`/Engine/EditorBlueprintResources/StandardMacros.IsValid` _found
    (:`Is Valid`
      (`Actor.K2_SetActorTransform` _found SpawnTransform false false)
      (`/Game/Blueprints/Misc/BP_PoolActor.SetInUse` _found true Lifetime)
      (return _found))))