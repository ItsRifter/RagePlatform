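; BP_PoolActor is a poolable actor that switches between active and dormant states for reuse, starting dormant on BeginPlay.
; SetInUse stores the state, toggles collision, visibility and tick together, and clears any running lifetime timer.
; When activated, it starts a new timer for the given lifetime, which fires ReturnToPool to deactivate the actor instead of destroying it.
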(event `self.ReceiveBeginPlay`
  (`self.SetInUse` false))

(event `SetInUse`
  (params (SetUse :type Boolean) (Lifetime :type "Float (double-precision)" :default 1.0))
  (set `self.InUse` SetUse)
  (`self.SetActorEnableCollision` SetUse)
  (`self.SetActorHiddenInGame` (not SetUse))
  (`self.SetActorTickEnabled` SetUse)
  (`KismetSystemLibrary.K2_ClearAndInvalidateTimerHandle` (`self.ObjectLifeTimer`))
  (if SetUse
    (bind _returnvalue (`KismetSystemLibrary.K2_SetTimerDelegate` (delegate `ReturnToPool`) Lifetime))
    (set `self.ObjectLifeTimer` _returnvalue)))

(event `ReturnToPool`
  (`self.SetInUse` false))

(fn `UserConstructionScript`)