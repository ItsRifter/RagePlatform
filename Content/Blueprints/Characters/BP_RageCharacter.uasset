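; Player character for a trap-filled, multi-level game, handling death presentation, restart, level start and saving.
; Trap type selects the ABP_Player death animation, falls hand the view to an impulse-driven temp camera, and timelines drive drowning and look-at camera moves.
; RGameInstance restart events clear those effects and revive the player.
; Level start fades in and enables timers; game close saves progress, while SaveGame stores player stats and deletes that progress.
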(event `LookAtTarget`
  (params (Actor :type "Actor Object Reference") (LocOffset :type "Vector Structure"))
  (bind _camera (`self.Camera`))
  ; Look at target with vector offset
  (`SceneComponent.SetVisibility` (`self.Mesh`) false false)
  (set `CameraComponent.bUsePawnControlRotation` false _camera)
  (`Timeline|Timeline_0` :!via `PlayFromStart`
    (:`Update`
      (`SceneComponent.K2_SetWorldRotation` (`self.Camera`) (`KismetMathLibrary.RInterpTo` (`SceneComponent.K2_GetComponentRotation` _camera) (`KismetMathLibrary.FindLookAtRotation` (`SceneComponent.K2_GetComponentLocation` _camera) (+ LocOffset (`self.K2_GetActorLocation` Actor))) 0.2 0.3) false false))))

(event `self.PlayerFall`
  (params (Impulse :type "Vector Structure"))
  ;[0.02604 0.02604 0.02604 0.5] Player Fall Impact
  (`/Engine/EditorBlueprintResources/StandardMacros.DoOnce` false :!label _label
    (:`Completed`
      (bind _returnvalue (`|SpawnActorFromClass` "/Game/Blueprints/Traps/BP_TempCamera.BP_TempCamera_C" (`SceneComponent.K2_GetComponentToWorld` (`self.Camera`)) "Undefined" "MultiplyWithRoot" null null))
      (bind _output_get (set `self.Temp_Camera` _returnvalue))
      (`PlayerController.SetViewTargetWithBlend` (`GameplayStatics.GetPlayerController` 0) _output_get 0.0 "VTBlend_Linear" 0.0 false)
      (`PrimitiveComponent.AddImpulse` (`RTempCamera.Sphere` _output_get) Impulse "None" true))))

(event `ResetPlayerFall`
  ;[0.02604 0.02604 0.02604 0.5] Player Fall Impact
  (goto _label :!via `Reset`))

(event `self.ReceiveBeginPlay`
  (bind (_relativelocation_x _relativelocation_y _relativelocation_z) (`KismetMathLibrary.BreakVector` (`SceneComponent.RelativeLocation` (`self.Camera`))))
  ;[0.01722 0.15 0 0.5] Player spawn + setup
  (`|ExecutionSequence`
    (:`then_0`
      (bind _asrgame_instance (cast `RGameInstance` (`GameplayStatics.GetGameInstance`))
        (:`then`
          (bind _output_get (set `self.RGameInstance` _asrgame_instance))
          (add `RGameInstance.OnGameRestart` _output_get (delegate `ResetFadeEffect`))
          (add `RGameInstance.OnGameClosed` (`self.RGameInstance`) (delegate `OnGameClosed_Event`)))
        (:`CastFailed`
          _))
      (set `self.OrgCamHeight` _relativelocation_z)
      (`self.ResettingPlayer`)
      (`self.SetupWidgets`)
      (`self.LevelStartFade`))
    (:`then_1`
      (`self.GameInstance LevelStorage`))))

(event `self.DrownPlayer`
  (params (HitLocation :type "Vector Structure"))
  ;[0.02604 0.02604 0.02604 0.5] Handling Drowning
  (bind _returnvalue (`GameplayStatics.SpawnEmitterAtLocation` "/Game/StarterContent/Particles/P_Smoke.P_Smoke" HitLocation))
  (set `self.SmokeEffect` _returnvalue)
  (bind (_direction _newtrack_0) (`Timeline|Timeline` :!via `PlayFromStart`)
    (:`Update`
      (`SceneComponent.K2_SetRelativeLocation` (`self.Camera`) (`KismetMathLibrary.VLerp` (0.0 20.0 145.0) (0.0 20.0 -145.0) _newtrack_0) false false))))

(event `ResetFadeEffect`
  ;[0.01722 0.15 0 0.5] Player spawn + setup
  (`/Game/Blueprints/UI/WB_FadeToBlack.ResetFade` (`self.FadeWidget`)))

(event `OnGameClosed_Event`
  ;[0.01722 0.15 0 0.5] Player spawn + setup
  (`self.Save Game Progress`))

(event `ResetLookAtTarget`
  (set `CameraComponent.bUsePawnControlRotation` true (`self.Camera`))
  (`SceneComponent.SetVisibility` (`self.Mesh`) true false))

(event `SetupWidgets`
  ; UI Widgets
  (bind _returnvalue (`|CreateWidget` "/Game/Blueprints/UI/WB_FadeToBlack.WB_FadeToBlack_C"))
  (bind _output_get (set `self.FadeWidget` _returnvalue))
  (`UserWidget.AddToViewport` _output_get -1))

(event `self.Respawn`
  ; Respawn
  (`SceneComponent.K2_SetRelativeLocation` (`self.Camera`) (`KismetMathLibrary.MakeVector` 0.0 20.0 (`self.OrgCamHeight`)) false false))

(event `ResettingPlayer`
  ;[0.02604 0.02604 0.02604 0.5] Reset Trigger
  (bind _asrgame_instance (cast `RGameInstance` (`GameplayStatics.GetGameInstance`)))
  (add `RGameInstance.OnGameRestart` _asrgame_instance (delegate `OnGameRestart_Event`)))

(event `PlayFadeEffect`
  (params (PlayRate :type "Float (double-precision)" :default 1.0))
  ; Fading
  (`/Game/Blueprints/UI/WB_FadeToBlack.FadeToBlack` (`self.FadeWidget`) PlayRate))

(event `FreezePlayer`
  ; Freeze/Unfreeze
  (set `RGameInstance.bCanLook` false (`self.RGameInstance`))
  (set `self.bRestrictKeyboard` true))

(event `OnGameRestart_Event`
  (bind _smokeeffect (`self.SmokeEffect`))
  (bind _temp_camera (`self.Temp_Camera`))
  ;[0.02604 0.02604 0.02604 0.5] Reset Trigger
  (`|ExecutionSequence`
    (:`then_0`
      (`TimelineComponent.Stop` (`self.Timeline`))
      (`/Engine/EditorBlueprintResources/StandardMacros.IsValid` _smokeeffect
        (:`Is Valid`
          (`ActorComponent.K2_DestroyComponent` _smokeeffect))))
    (:`then_1`
      (`/Engine/EditorBlueprintResources/StandardMacros.IsValid` _temp_camera
        (:`Is Valid`
          (`self.K2_DestroyActor` _temp_camera)
          (`PlayerController.SetViewTargetWithBlend` (`GameplayStatics.GetPlayerController` 0) self 0.0 "VTBlend_Linear" 0.0 false)
          (`self.ResetPlayerFall`))))
    (:`then_2`
      (bind _asabp_player (cast `/Game/Blueprints/Animation/Player/ABP_Player` (`SkeletalMeshComponent.GetAnimInstance` (`self.Mesh`))))
      (`/Game/Blueprints/Animation/Player/ABP_Player.Revive` _asabp_player))))

(event `UnfreezePlayer`
  ; Freeze/Unfreeze
  (set `RGameInstance.bCanLook` true (`self.RGameInstance`))
  (set `self.bRestrictKeyboard` false))

(event `self.OnDeath`
  (params (TrapEnum :type "ETrap Enum" :default "Spikes"))
  ;[0.8156 0.01498 0 0.5] Death animations
  (bind _asabp_player (cast `/Game/Blueprints/Animation/Player/ABP_Player` (`SkeletalMeshComponent.GetAnimInstance` (`self.Mesh`))))
  (switch `ETrap` TrapEnum
    (:`Spikes`
      (set `/Game/Blueprints/Animation/Player/ABP_Player.DeathType` "NewEnumerator0" _asabp_player :!label _label_2)
      (`/Game/Blueprints/Animation/Player/ABP_Player.DiedABP` _asabp_player))
    (:`Axe`
      (goto _label_2))
    (:`Saw`
      (goto _label_2))
    (:`Chandelier`
      (goto _label_2))
    (:`LavaPit`
      (set `/Game/Blueprints/Animation/Player/ABP_Player.DeathType` "NewEnumerator2" _asabp_player :!label _label_3)
      (`/Game/Blueprints/Animation/Player/ABP_Player.DiedABP` _asabp_player))
    (:`PoisonPit`
      (goto _label_3))
    (:`Explosion`
      (set `/Game/Blueprints/Animation/Player/ABP_Player.DeathType` "NewEnumerator1" _asabp_player)
      (`/Game/Blueprints/Animation/Player/ABP_Player.DiedABP` _asabp_player))
    (:`Arrows`
      (goto _label_2))))

(event `LevelStartFade`
  (bind _returnvalue (`GameplayStatics.GetGameInstance`))
  ;[0.026 0.026 0.026 0.5] Level Start Defaults and Fade
  (`/Engine/EditorBlueprintResources/StandardMacros.IsValid` (`GameplayStatics.GetPlayerController` 0)
    (:`Is Valid`
      (`PlayerCameraManager.StartCameraFade` :`self` (`PlayerController.PlayerCameraManager` (`GameplayStatics.GetPlayerController` 0)) :`FromAlpha` 1.0 :`ToAlpha` 1.0 :`Duration` 0.1 :`bHoldWhenFinished` true)
      (set `CharacterMovementComponent.MaxAcceleration` 0.0 (`Character.CharacterMovement` (`GameplayStatics.GetPlayerCharacter` 0)))
      (`KismetSystemLibrary.Delay` 1.0)
      (`PlayerCameraManager.StartCameraFade` :`self` (`PlayerController.PlayerCameraManager` (`GameplayStatics.GetPlayerController` 0)) :`FromAlpha` 1.0 :`Duration` 0.5)
      (`KismetSystemLibrary.Delay` 0.7)
      (set `CharacterMovementComponent.MaxAcceleration` 3072.0 (`Character.CharacterMovement` (`GameplayStatics.GetPlayerCharacter` 0)))
      (`/Engine/EditorBlueprintResources/StandardMacros.IsValid` _returnvalue
        (:`Is Valid`
          (bind _asrgame_instance (cast `RGameInstance` _returnvalue))
          (bind _returnvalue_2 (`GameplayStatics.GetCurrentLevelName` true))
          (if (`KismetStringLibrary.Contains` _returnvalue_2 "Level1")
            (set `RGameInstance.GameTimeVar` 0.0 _asrgame_instance))
          (set `RGameInstance.TimeVar` 0.0 _asrgame_instance)
          (set `RGameInstance.bCanCountLevelTime` true _asrgame_instance)
          (set `RGameInstance.bCanCountGameTime` true _asrgame_instance)
          (set `RGameInstance.bCanLook` true _asrgame_instance)
          (set `RGameInstance.bCanPause` true _asrgame_instance))))))

(event `EnhancedInput|/Game/Blueprints/Inputs/IA_SkipDialogue`
  (params (ActionValue :type Boolean) (ElapsedSeconds :type "Float (double-precision)") (TriggeredSeconds :type "Float (double-precision)") (InputAction :type "InputAction Object Reference" :default "/Game/Blueprints/Inputs/IA_SkipDialogue.IA_SkipDialogue"))
  ; Skip Dialogue
  (:`Triggered`
    (`self.RequestSkipDialogue`)))

(event `self.SaveGame`
  (params (PlayerStats :type "PlayerStats Structure"))
  (bind _player_stats_playername (break `PlayerStats` (`self.Player Stats`)))
  (bind _playerstats (`/Game/Blueprints/Saves/BP_Saves.PlayerStats` (`self.SavedGame`)))
  (`|ExecutionSequence`
    (:`then_0`
      (bind _output_get (set `self.Player Stats` PlayerStats))
      (bind _returnvalue (`GameplayStatics.DoesSaveGameExist` "Slot1"))
      (if _returnvalue
        (bind _returnvalue_2 (`GameplayStatics.LoadGameFromSlot` "Slot1"))
        (bind _asbp_saves (cast `/Game/Blueprints/Saves/BP_Saves` _returnvalue_2))
        (set `self.SavedGame` _asbp_saves)
        (for _array_element _playerstats
          (if (`KismetStringLibrary.EqualEqual_StrStr` (`.PlayerName` (break `PlayerStats` _array_element)) _player_stats_playername)
            (`|ExecutionSequence`
              (:`then_0`
                (break))
              (:`then_1`
                (`KismetArrayLibrary.Array_RemoveItem` _playerstats _array_element)))))
        (`KismetArrayLibrary.Array_Add` _playerstats (`self.Player Stats`))
        (else
          (bind _returnvalue_3 (`GameplayStatics.CreateSaveGameObject` "/Game/Blueprints/Saves/BP_Saves.BP_Saves_C"))
          (bind _output_get_2 (set `self.SavedGame` _returnvalue_3))
          (`KismetArrayLibrary.Array_Add` (`/Game/Blueprints/Saves/BP_Saves.PlayerStats` _output_get_2) _output_get)))
      (`GameplayStatics.SaveGameToSlot` _output_get_2 "Slot1"))
    (:`then_1`
      (bind _returnvalue_4 (`GameplayStatics.DoesSaveGameExist` "GameProgress"))
      (if _returnvalue_4
        (`GameplayStatics.DeleteGameInSlot` "GameProgress")))))

(event `GameInstance LevelStorage`
  (`/Engine/EditorBlueprintResources/StandardMacros.IsValid` (`self.RGameInstance`)
    (:`Is Valid`
      (bind _returnvalue (`GameplayStatics.GetCurrentLevelName` true))
      (set `RGameInstance.LevelName` (`KismetStringLibrary.Conv_StringToName` _returnvalue) (`self.RGameInstance`))
      (switch `string` _returnvalue
        (:`Level1`
          (set `RGameInstance.LevelNumber` 1 (`self.RGameInstance`)))
        (:`Level2`
          (set `RGameInstance.LevelNumber` 2 (`self.RGameInstance`)))
        (:`Level3`
          (set `RGameInstance.LevelNumber` 3 (`self.RGameInstance`)))
        (:`Level4`
          (set `RGameInstance.LevelNumber` 4 (`self.RGameInstance`)))
        (:`Level5`
          (set `RGameInstance.LevelNumber` 5 (`self.RGameInstance`)))
        (:`LevelEnd`
          (set `RGameInstance.LevelNumber` 6 (`self.RGameInstance`)))))))

(event `Save Game Progress`
  (bind _rgameinstance (`self.RGameInstance`))
  (`/Engine/EditorBlueprintResources/StandardMacros.IsValid` (`self.RGameInstance`)
    (:`Is Valid`
      (bind _returnvalue (`GameplayStatics.DoesSaveGameExist` "GameProgress"))
      (if _returnvalue
        (`GameplayStatics.DeleteGameInSlot` "GameProgress"))
      (bind _returnvalue_2 (`GameplayStatics.CreateSaveGameObject` "/Game/Blueprints/Saves/BP_GameProgress.BP_GameProgress_C"))
      (set `/Game/Blueprints/Saves/BP_GameProgress.LastLevelReached` (`RGameInstance.LevelName` _rgameinstance) _returnvalue_2)
      (set `/Game/Blueprints/Saves/BP_GameProgress.PlayerStatsOld` (`RGameInstance.PlayerStats` _rgameinstance) _returnvalue_2)
      (set `/Game/Blueprints/Saves/BP_GameProgress.GameTimeVar` (`RGameInstance.GameTimeVar` _rgameinstance) _returnvalue_2)
      (set `/Game/Blueprints/Saves/BP_GameProgress.Deaths` (`RGameInstance.DeathCount` _rgameinstance) _returnvalue_2)
      (set `/Game/Blueprints/Saves/BP_GameProgress.LevelTime` (`RGameInstance.TimeVar` _rgameinstance) _returnvalue_2)
      (`GameplayStatics.SaveGameToSlot` _returnvalue_2 "GameProgress"))))

(fn `UserConstructionScript`)